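; Manager Blueprint for the Invo SDK, wrapping its web API for auth, balances, currency purchases, sends, transfers, items and game lookups.
; Each event issues an InvoRequest using game-secret, Authorization or blank headers; most print the result, some cache JSON fields.
; BeginPlay logs in with a hard-coded password, checks balance, then fetches dashboard game names after a fixed delay.
; Other EventGraph calls are unwired, and several endpoints hard-code IDs or query values.
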(event `self.ReceiveBeginPlay`
  (`self.Invo Login` (`self.PlayerEmail`) "Welcome@2020")
  (`self.Player Balance Check` (`self.PlayerEmail`))
  (`KismetSystemLibrary.Delay` 2.0)
  (`self.Invo Games Dashboard Full Data`))

(event `Invo Register Initiate`
  (params (`First Name` :type String) (`Last Name` :type String) (Email :type String) (`User Type` :type String) (`Accepted Terms` :type Boolean))
  ;[0 0 0] Auth
  ;;[1 1 1] Register
  (bind _responsecontent (`InvoSDKApiManager.InvoRequest` (`self.Base Url`) "auth/register/initiate?Content-Type=application/json" (`|MakeMap` "") (`self.FormatBody` (`|FormatText` "    \"first_name\": \"{First Name}\", \n    \"last_name\": \"{Last Name}\", \n    \"email\": \"{Email}\", \n    \"user_type\": \"{User Type}\", \n    \"accepted_terms\": {Terms}" `First Name` `Last Name` Email `User Type` `Accepted Terms`)) "POST")
    (:`OnSuccess`
      (`KismetSystemLibrary.PrintString` "Success" true true (struct :`G` 1.0 :`A` 1.0))
      (`KismetSystemLibrary.PrintString` _responsecontent))
    (:`OnFail`
      (`KismetSystemLibrary.PrintString` "Failed" true true (struct :`R` 1.0 :`A` 1.0))
      (`KismetSystemLibrary.PrintString` _responsecontent))))

(event `Invo Login`
  (params (Email :type String) (Password :type String))
  ;[0 0 0] Auth
  ;;[1 1 1] Login
  (bind (_responsecontent _statuscode _bwassuccessful _jsonobject) (`InvoSDKApiManager.InvoRequest` (`self.Base Url`) "auth/login" (`|MakeMap` "") (`self.FormatBody` (`|FormatText` "    \"email\": \"{Email}\", \n    \"password\": \"{Password}\"" Email Password)) "POST")
    (:`OnSuccess`
      (`KismetSystemLibrary.PrintString` "Success" true true (struct :`G` 1.0 :`A` 1.0))
      (`KismetSystemLibrary.PrintString` _responsecontent)
      (set `self.Token` (`InvoSDKJsonHelpers.GetStringField` _jsonobject "access_token")))
    (:`OnFail`
      (`KismetSystemLibrary.PrintString` "Failed" true true (struct :`R` 1.0 :`A` 1.0))
      (`KismetSystemLibrary.PrintString` _responsecontent))))

(event `Invo Verify Pin`
  (params (Email :type String) (PIN :type Integer))
  ;[0 0 0] Auth
  ;;[1 1 1] Invo Verify Pin
  (bind _responsecontent (`InvoSDKApiManager.InvoRequest` (`self.Base Url`) "auth/verify-pin" (`|MakeMap` "") (`self.FormatBody` (`|FormatText` "    \"email\": \"{Email}\", \n    \"pin\": \"{PIN}\"" Email PIN)) "POST")
    (:`OnSuccess`
      (`KismetSystemLibrary.PrintString` "Success" true true (struct :`G` 1.0 :`A` 1.0))
      (`KismetSystemLibrary.PrintString` _responsecontent))
    (:`OnFail`
      (`KismetSystemLibrary.PrintString` "Failed" true true (struct :`R` 1.0 :`A` 1.0))
      (`KismetSystemLibrary.PrintString` _responsecontent))))

(event `Player Purchase Currency Function`
  (params (`Player Email` :type String) (`Player Name` :type String) (`Player Phone` :type String) (`USD Amount` :type Integer) (`Purchase Reference` :type String) (`Payment Method ID` :type String) (`Save Card` :type Boolean))
  ;[0 0 0] Purchase
  ;;[1 1 1] Player Purchase Currency Function
  (`InvoSDKApiManager.InvoRequest` (`self.Base Url`) "api/currency-purchases/purchase-currency" (`|MakeMap` "X-Game-Secret-Key" (`self.X-Game-Secret-Key`)) (`self.FormatBody` (`|FormatText` "    \"player_email\": \"{Player Email}\", \n    \"player_name\": \"{Player Name}\", \n    \"player_phone\": \"{Player Phone}\", \n    \"usd_amount\": \"{USD Amount}\", \n    \"purchase_reference\": \"{Purchase Reference}\", \n    \"payment_method_id\": \"{Payment Method ID}\", \n    \"save_card\": {Save Card}" `Player Email` `Player Name` `Player Phone` `USD Amount` `Purchase Reference` `Payment Method ID` `Save Card`)) "POST"
    (:`OnSuccess`
      (`KismetSystemLibrary.PrintString` "Success" true true (struct :`G` 1.0 :`A` 1.0)))
    (:`OnFail`
      (`KismetSystemLibrary.PrintString` "Failed" true true (struct :`R` 1.0 :`A` 1.0)))))

(event `Transfers Verify SMS`
  (params (TransactionID :type String) (`SMS PIN` :type Integer))
  ;[0 0 0] Transfer Events
  ;;[1 1 1] Transfers Verify SMS
  (`InvoSDKApiManager.InvoRequest` (`self.Base Url`) "api/transfers/verify-sms" (`|MakeMap` "X-Game-Secret-Key" (`self.X-Game-Secret-Key`)) (`self.FormatBody` (`|FormatText` "    \"transaction_id\": \"{Transaction ID}\", \n    \"sms_pin\": \"{SMS PIN}\"" TransactionID `SMS PIN`)) "POST"
    (:`OnSuccess`
      (`KismetSystemLibrary.PrintString` "Success" true true (struct :`G` 1.0 :`A` 1.0)))
    (:`OnFail`
      (`KismetSystemLibrary.PrintString` "Failed" true true (struct :`R` 1.0 :`A` 1.0)))))

(event `Currency Sends Initiate Send`
  (params (`Client Transfer ID` :type String) (`Sender Name ` :type String) (`Sender Email ` :type String) (`Sender Phone ` :type String) (`Receiver Phone` :type String) (`Receiver Game ID` :type String) (`Amount ` :type Integer))
  ;[0 0 0] Currency Events
  ;;[1 1 1] Currency Sends Initiate Send
  (`InvoSDKApiManager.InvoRequest` (`self.Base Url`) "api/currency-sends/initiate-send" (`|MakeMap` "X-Game-Secret-Key" (`self.X-Game-Secret-Key`)) (`self.FormatBody` (`|FormatText` "  \"client_request_id\": \"{Client Request ID}\", \n  \"sender_player_name\": \"{Sender Name}\", \n  \"sender_player_email\": \"{Sender Email}\", \n  \"sender_player_phone\": \"{Sender Phone}\", \n  \"receiver_player_phone\": \"{Receiver Phone}\", \n  \"receiving_game_id\": \"{Receiving Game ID}\", \n  \"amount\": \"{Amount}\"" `Client Transfer ID` `Sender Name ` `Sender Email ` `Sender Phone ` `Receiver Phone` `Receiver Game ID` `Amount `)) "POST"
    (:`OnSuccess`
      (`KismetSystemLibrary.PrintString` "Success" true true (struct :`G` 1.0 :`A` 1.0)))
    (:`OnFail`
      (`KismetSystemLibrary.PrintString` "Failed" true true (struct :`R` 1.0 :`A` 1.0)))))

(event `Transfers Initiate Transfer`
  (params (`Client Transfer ID` :type String) (`Source Player Name ` :type String) (`Source Player Email ` :type String) (`Source Player Phone ` :type String) (`Target Game ID ` :type String) (`Amount ` :type Integer))
  ;[0 0 0] Transfer Events
  ;;[1 1 1] Transfers Initiate Transfer
  (`InvoSDKApiManager.InvoRequest` (`self.Base Url`) "api/transfers/initiate-transfer" (`|MakeMap` "X-Game-Secret-Key" (`self.X-Game-Secret-Key`)) (`self.FormatBody` (`|FormatText` "    \"client_request_id\": \"{Client Transfer ID}\", \n    \"source_player_name\": \"{Name}\", \n    \"source_player_email\": \"{Email}\", \n    \"source_player_phone\": \"{Phone}\", \n    \"target_game_id\": \"{Game ID}\", \n    \"amount\": \"{Amount}\"" `Client Transfer ID` `Source Player Name ` `Source Player Email ` `Source Player Phone ` `Target Game ID ` `Amount `)) "POST"
    (:`OnSuccess`
      (`KismetSystemLibrary.PrintString` "Success" true true (struct :`G` 1.0 :`A` 1.0)))
    (:`OnFail`
      (`KismetSystemLibrary.PrintString` "Failed" true true (struct :`R` 1.0 :`A` 1.0)))))

(event `Currency Sends Verify Sms`
  (params (Email :type String) (PIN :type Integer))
  ;[0 0 0] Currency Events
  ;;[1 1 1] Currency Sends Verify Sms
  (`InvoSDKApiManager.InvoRequest` (`self.Base Url`) "api/currency-sends/verify-sms" (`|MakeMap` "X-Game-Secret-Key" (`self.X-Game-Secret-Key`)) (`self.FormatBody` (`|FormatText` "    \"transaction_id\": \"{Transaction ID}\", \n    \"sms_pin\": \"{SMS PIN}\"" Email PIN)) "POST"
    (:`OnSuccess`
      (`KismetSystemLibrary.PrintString` "Success" true true (struct :`G` 1.0 :`A` 1.0)))
    (:`OnFail`
      (`KismetSystemLibrary.PrintString` "Failed" true true (struct :`R` 1.0 :`A` 1.0)))))

(event `Transfers Claim Transfer`
  (params (`Claim Code ` :type String) (`Target Player Name ` :type String) (`Target Player Email ` :type String) (`Target Player Phone ` :type String) (`Target Currency ID ` :type String))
  ;[0 0 0] Transfer Events
  ;;[1 1 1] Transfers Claim Transfer
  (`InvoSDKApiManager.InvoRequest` (`self.Base Url`) "api/transfers/claim-transfer" (`|MakeMap` "X-Game-Secret-Key" (`self.X-Game-Secret-Key`)) (`self.FormatBody` (`|FormatText` "    \"claim_code\": \"{Claim Code}\", \n    \"target_player_name\": \"{Name}\", \n    \"target_player_email\": \"{Email}\", \n    \"target_player_phone\": \"{Phone}\", \n    \"target_currency_id\": \"{Currency ID}\"" `Claim Code ` `Target Player Name ` `Target Player Email ` `Target Player Phone ` `Target Currency ID `)) "POST"
    (:`OnSuccess`
      (`KismetSystemLibrary.PrintString` "Success" true true (struct :`G` 1.0 :`A` 1.0)))
    (:`OnFail`
      (`KismetSystemLibrary.PrintString` "Failed" true true (struct :`R` 1.0 :`A` 1.0)))))

(event `Currency Sends Claim Currency`
  (params (`Claim Code ` :type String) (`Receiver Name` :type String) (`Receiver Email` :type String) (`Receiver Phone` :type String) (`Receiver CurrencyID ` :type Integer))
  ;[0 0 0] Currency Events
  ;;[1 1 1] Currency Sends Claim Currency
  (`InvoSDKApiManager.InvoRequest` (`self.Base Url`) "api/currency-sends/claim-currency" (`|MakeMap` "X-Game-Secret-Key" (`self.X-Game-Secret-Key`)) (`self.FormatBody` (`|FormatText` "    \"claim_code\": \"{Claim Code}\", \n    \"receiver_player_name\": \"{Name}\", \n    \"receiver_player_email\": \"{Email}\", \n    \"receiver_player_phone\": \"{Phone}\", \n    \"receiver_currency_id\": \"{Currency ID}\"" `Claim Code ` `Receiver Name` `Receiver Email` `Receiver Phone` `Receiver CurrencyID `)) "POST"
    (:`OnSuccess`
      (`KismetSystemLibrary.PrintString` "Success" true true (struct :`G` 1.0 :`A` 1.0)))
    (:`OnFail`
      (`KismetSystemLibrary.PrintString` "Failed" true true (struct :`R` 1.0 :`A` 1.0)))))

(event `Invo Games Dashboard Full Data`
  ;[1 1 1] Invo Games Dashboard Full Data
  (bind (_responsecontent _statuscode _bwassuccessful _jsonobject) (`InvoSDKApiManager.InvoRequest` (`self.Base Url`) "api/games/dashboard/full-data?Content-Type=application/json" (`self.Authorization`) "" "GET")
    (:`OnSuccess`
      (`KismetSystemLibrary.PrintString` "Success" true true (struct :`G` 1.0 :`A` 1.0))
      (for _array_element (`InvoSDKJsonHelpers.GetObjectsArray` _jsonobject "games")
        (`KismetArrayLibrary.Array_AddUnique` (`self.Games`) (`InvoSDKJsonHelpers.GetStringField` _array_element "game_name"))))
    (:`OnFail`
      (`KismetSystemLibrary.PrintString` "Failed" true true (struct :`R` 1.0 :`A` 1.0)))))

(event `Invo Games Lookup By ID`
  ;[1 1 1] Invo Games Lookup By ID
  (`InvoSDKApiManager.InvoRequest` (`self.Base Url`) "api/games/306720264148/analytics?range=24h" (`self.Authorization`) "" "GET"
    (:`OnSuccess`
      (`KismetSystemLibrary.PrintString` "Success" true true (struct :`G` 1.0 :`A` 1.0)))
    (:`OnFail`
      (`KismetSystemLibrary.PrintString` "Failed" true true (struct :`R` 1.0 :`A` 1.0)))))

(event `Player Balance Check`
  (params (`Player Email` :type String))
  ;[1 1 1] PlayerBalanceCheck
  (bind (_responsecontent _statuscode _bwassuccessful _jsonobject) (`InvoSDKApiManager.InvoRequest` (`self.Base Url`) (`KismetStringLibrary.Concat_StrStr` "api/player-balances/player/by-email/" `Player Email`) (`|MakeMap` "X-Game-Secret-Key" (`self.X-Game-Secret-Key`)) "" "GET")
    (:`OnSuccess`
      (`KismetSystemLibrary.PrintString` "Success" true true (struct :`G` 1.0 :`A` 1.0))
      (set `self.AmountRecieved?` _bwassuccessful)
      (bind _output (`|GetArrayItem` (`InvoSDKJsonHelpers.GetObjectsArray` _jsonobject "balances")))
      (set `self.AvailableBalance` (`InvoSDKJsonHelpers.GetIntegerField` _output "available_balance"))
      (set `self.CurrencyName` (`InvoSDKJsonHelpers.GetStringField` _output "currency_name")))
    (:`OnFail`
      (`KismetSystemLibrary.PrintString` "Failed" true true (struct :`R` 1.0 :`A` 1.0)))))

(event `Invo Users Games`
  ;[1 1 1] Invo Users Games
  (`InvoSDKApiManager.InvoRequest` (`self.Base Url`) "api/users/22/games" (`self.Authorization`) "" "GET"
    (:`OnSuccess`
      (`KismetSystemLibrary.PrintString` "Success" true true (struct :`G` 1.0 :`A` 1.0)))
    (:`OnFail`
      (`KismetSystemLibrary.PrintString` "Failed" true true (struct :`R` 1.0 :`A` 1.0)))))

(event `Player Purchase History`
  (params (`Player Email` :type String) (Limit :type Integer))
  ;[1 1 1] Player Purchase History
  (bind (_responsecontent _statuscode _bwassuccessful _jsonobject) (`InvoSDKApiManager.InvoRequest` (`self.Base Url`) "api/currency-purchases/player-purchase-history?player_email=atrhick@hotmail.com&limit=10&offset=0" (`|MakeMap` "X-Game-Secret-Key" (`self.X-Game-Secret-Key`)) "" "GET")
    (:`OnSuccess`
      (`KismetSystemLibrary.PrintString` "Success" true true (struct :`G` 1.0 :`A` 1.0))
      (set `self.Purchase History Json Object` _jsonobject))
    (:`OnFail`
      (`KismetSystemLibrary.PrintString` "Failed" true true (struct :`R` 1.0 :`A` 1.0)))))

(event `Invo Generate Upload URL`
  (params (FileName :type String))
  ;[1 1 1] Invo Generate Upload URL
  (`InvoSDKApiManager.InvoRequest` (`self.Base Url`) "api/generate-avatar-upload-url" (`|MakeMap` "") (`self.FormatBody` (`|FormatText` "    \"filename\": \"{File Name}\", \n    \"contentType\": \"image/png\"" FileName)) "POST"
    (:`OnSuccess`
      (`KismetSystemLibrary.PrintString` "Success" true true (struct :`G` 1.0 :`A` 1.0)))
    (:`OnFail`
      (`KismetSystemLibrary.PrintString` "Failed" true true (struct :`R` 1.0 :`A` 1.0)))))

(event `Item Purchases Purchase Items`
  (params (`Client Request ID` :type String) (`Player Email` :type String) (`Player Name` :type String) (`Item ID` :type String) (`Item Name` :type String) (`Item Quantity` :type Integer) (`Unit Price` :type Integer) (`Total Price` :type Integer))
  ;[1 1 1] Item Purchases Purchase Item
  (`InvoSDKApiManager.InvoRequest` (`self.Base Url`) "api/item-purchases/purchase-item" (`|MakeMap` "X-Game-Secret-Key" (`self.X-Game-Secret-Key`)) (`self.FormatBody` (`|FormatText` "  \"client_request_id\": \"{Client Request ID}\", \n  \"player_email\": \"{Player Email}\", \n  \"player_name\": \"{Player Name}\", \n  \"item_id\": \"{Item ID}\", \n  \"item_name\": \"{Item Name}\", \n  \"item_quantity\": {Item Quantity}, \n  \"unit_price\": \"{Unit Price}\", \n  \"total_price\": \"{Total Price}\"" `Client Request ID` `Player Email` `Player Name` `Item ID` `Item Name` `Item Quantity` `Unit Price` `Total Price`)) "POST"
    (:`OnSuccess`
      (`KismetSystemLibrary.PrintString` "Success" true true (struct :`G` 1.0 :`A` 1.0)))
    (:`OnFail`
      (`KismetSystemLibrary.PrintString` "Failed" true true (struct :`R` 1.0 :`A` 1.0)))))

(event `GetItemList`
  ;[1 1 1] Get Item List
  (bind (_responsecontent _statuscode _bwassuccessful _jsonobject) (`InvoSDKApiManager.InvoRequest` (`self.Base Url`) "api/v1/game-items/list" (`|MakeMap` "") (`self.FormatBody` (`|FormatText` "\"game_secret\": \"{GameSecret}\"" (`self.X-Game-Secret-Key`))) "POST")
    (:`OnSuccess`
      (`KismetSystemLibrary.PrintString` "Success" true true (struct :`G` 1.0 :`A` 1.0))
      (set `self.Item List Json Object` _jsonobject))
    (:`OnFail`
      (`KismetSystemLibrary.PrintString` "Failed" true true (struct :`R` 1.0 :`A` 1.0)))))

(fn `UserConstructionScript`)